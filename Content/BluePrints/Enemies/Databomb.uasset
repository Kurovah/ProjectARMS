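; Databomb is an enemy that tumbles in place and flickers when the player mech comes near.
; BeginPlay picks a random rotation step that Tick applies to the mesh, and a DetectSphere overlap starts a permanent flicker alternating mesh scale through a FlipFlop and short Delay.
; Tick also rebinds the child HurtBox's hit event, which destroys the actor.
; The attack only sets the flicker, with no explosion or damage here.
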(event `self.ReceiveBeginPlay`
  (set `self.Delta Rotation` (`KismetMathLibrary.MakeRotator` (`KismetMathLibrary.RandomFloat`) (`KismetMathLibrary.RandomFloat`) (`KismetMathLibrary.RandomFloat`))))

(event `self.ReceiveTick`
  (params (DeltaSeconds :type "Float (single-precision)"))
  (bind _ashurt_box (cast `/Game/Actors/HurtBox` (`ChildActorComponent.ChildActor` (`self.Hurtbox`))))
  (add `/Game/Actors/HurtBox.OnHit` _ashurt_box (delegate `HitLanded`))
  (`SceneComponent.K2_AddLocalRotation` (`self.Mesh`) (`self.Delta Rotation`) false false)
  (if (`self.flickering`)
    (`/Engine/EditorBlueprintResources/StandardMacros.FlipFlop`
      (:`A`
        (set `self.Meshscale` (1.0 1.0 1.0)))
      (:`B`
        (set `self.Meshscale` (0.8 0.8 0.8))))
    (`KismetSystemLibrary.Delay` 0.05)
    (`SceneComponent.SetWorldScale3D` (`self.Mesh`) (`self.Meshscale`))))

(event `AttackStart`
  (set `self.flickering` true))

(event `HitLanded`
  (params (HitContext :type "HitContext Structure"))
  (`self.K2_DestroyActor`))

(event `self.DetectSphere.OnComponentBeginOverlap`
  (params (OverlappedComponent :type "PrimitiveComponent Object Reference") (OtherActor :type "Actor Object Reference") (OtherComp :type "PrimitiveComponent Object Reference") (OtherBodyIndex :type Integer) (bFromSweep :type Boolean) (SweepResult :type "HitResult Structure (by ref)"))
  (cast `/Game/BluePrints/MechPlayerCharacterBP` OtherActor)
  (`self.AttackStart`))

(fn `UserConstructionScript`)