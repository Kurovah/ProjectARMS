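; Data Spider enemy that patrols, attacks the player, and dies when hit.
; Tick moves it forward until a short forward line trace finds nothing, then it pauses and flips on a timer.
; Player overlap plays an attack montage whose notify applies hits through a sphere overlap.
; A HurtBox child actor's hit event launches it along Y and up in low gravity, then a timer spawns defeat VFX and destroys it.
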(event `self.ReceiveBeginPlay`
  (`KismetArrayLibrary.Array_Add` (`self.Actors to Ignore`) (`GameplayStatics.GetPlayerCharacter` 0))
  (`self.StartMoving`)
  (bind _ashurt_box (cast `/Game/Actors/HurtBox` (`ChildActorComponent.ChildActor` (`self.hurtbox`))))
  (add `/Game/Actors/HurtBox.OnHit` _ashurt_box (delegate `Fly off`)))

(event `Fly off`
  (params (HitContext :type "HitContext Structure"))
  (bind (_sourceposition _damagevalue _launchvalue) (break `HitContext` HitContext))
  (set `self.isMoving` false)
  (set `CharacterMovementComponent.GravityScale` 0.2 (`self.CharacterMovement`))
  (`self.LaunchCharacter` (`KismetMathLibrary.MakeVector` 0.0 (.y (* (`KismetMathLibrary.Normal` (`KismetMathLibrary.MakeVector` 0.0 (`KismetMathLibrary.SignOfFloat` (- (.y (`self.K2_GetActorLocation`)) (.y _sourceposition))) 0.5)) _launchvalue)) (/ _launchvalue 2.0)) true true)
  (`self.PlayAnimMontage` "/Game/Meshes/enemies/DataSpider/Anims/DS_Defeated_Montage.DS_Defeated_Montage")
  (`KismetSystemLibrary.K2_SetTimerDelegate` (delegate `KillChar`) 1.0))

(event `KillChar`
  (`NiagaraFunctionLibrary.SpawnSystemAtLocation` "/Game/particle_systems/EnemyDefeat.EnemyDefeat" (.location (`self.GetTransform`)) (.rotation (`self.GetTransform`)))
  (`self.K2_DestroyActor`))

(event `flip`
  (`self.K2_SetActorRotation` (`KismetMathLibrary.ComposeRotators` (`self.K2_GetActorRotation`) (struct :`Yaw` 180.0))))

(event `FlipnMove`
  (`self.flip`)
  (`self.StartMoving`))

(event `StartMoving`
  (set `self.movement` 1.0)
  (set `self.isMoving` true))

(event `stopmoving`
  (set `self.movement` 0.0)
  (set `self.isMoving` false))

(event `self.ReceiveTick`
  (params (DeltaSeconds :type "Float (single-precision)"))
  (bind _returnvalue (`self.K2_GetActorLocation`))
  (if (`self.isMoving`)
    (`PawnMovementComponent.AddInputVector` (`self.CharacterMovement`) (* (`self.GetActorForwardVector`) (`self.movement`)) false)
    (bind (_outhit _returnvalue_2) (`KismetSystemLibrary.LineTraceSingleForObjects` _returnvalue (+ _returnvalue (* (`self.GetActorForwardVector`) 1.0)) (`self.Object Types`) false (`self.Actors to Ignore`) "ForOneFrame"))
    (if (not _returnvalue_2)
      (`self.stopmoving`)
      (`KismetSystemLibrary.K2_SetTimerDelegate` (delegate `FlipnMove`) 2.0))))

(event `self.Sphere.OnComponentBeginOverlap`
  (params (OverlappedComponent :type "PrimitiveComponent Object Reference") (OtherActor :type "Actor Object Reference") (OtherComp :type "PrimitiveComponent Object Reference") (OtherBodyIndex :type Integer) (bFromSweep :type Boolean) (SweepResult :type "HitResult Structure (by ref)"))
  (bind _returnvalue (+ (* (`self.GetActorForwardVector`) 100.0) (`self.K2_GetActorLocation`)))
  (cast `/Game/BluePrints/MechPlayerCharacterBP` OtherActor)
  (if (`self.canAttack`)
    (set `self.canAttack` false)
    (`self.stopmoving`)
    (`|PlayMontage` (`self.Mesh`) "/Game/Meshes/enemies/DataSpider/Anims/DS_Attack_Montage.DS_Attack_Montage"
      (:`OnCompleted`
        (set `self.canAttack` true)
        (`self.StartMoving`))
      (:`OnNotifyBegin`
        (bind _outactors (`KismetSystemLibrary.SphereOverlapActors` _returnvalue 100.0 (`self.Object Types_0`) "/Game/BluePrints/MechPlayerCharacterBP.MechPlayerCharacterBP_C"))
        (`KismetSystemLibrary.DrawDebugSphere` _returnvalue 100.0 12 (struct :`R` 1.0 :`G` 1.0 :`B` 1.0 :`A` 1.0) 1.0)
        (for _array_element _outactors
          (bind _asmech_player_character_bp (cast `/Game/BluePrints/MechPlayerCharacterBP` _array_element))
          (`MechPlayerCharacter.ApplyHit` _asmech_player_character_bp (make `HitContext` (`self.K2_GetActorLocation`) 1.0 1000.0)))))))

(fn `UserConstructionScript`)