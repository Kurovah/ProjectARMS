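; HitBoxManager spawns and clears attack hitboxes for the actor that owns it.
; CreateHitBox spawns a HitBox at an unrotated world-space offset from the owner, using its rotation and multiplied scale.
; Each hitbox receives its creator, launch power and damage, attaches to the owner and is tracked in an array.
; ClearHitboxes destroys tracked hitboxes but removes entries while iterating that array, which can skip some.
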(fn `ClearHitboxes`
  (locals (`actor to destroy` :type "/Game/Actors/HitBox Object Reference"))
  (bind _hitboxes (`self.HitBoxes`))
  (for _array_element _hitboxes
    (set `local.actor to destroy` _array_element)
    (`KismetArrayLibrary.Array_RemoveItem` _hitboxes _array_element)
    (`Actor.K2_DestroyActor` (`local.actor to destroy`))))

(fn `CreateHitBox`
  (params (PositionOffset :type "Vector Structure") (LaunchPower :type "Float (double-precision)") (AttackPower :type "Float (double-precision)") (ScaleMultiplier :type "Float (double-precision)"))
  (locals (Scalemultiply :type "Float (double-precision)" :default 1.0) (`Created HB` :type "/Game/Actors/HitBox Object Reference"))
  (bind _returnvalue (`self.GetOwner`))
  (set `local.Scalemultiply` ScaleMultiplier)
  (bind _returnvalue_2 (`|SpawnActorFromClass` "/Game/Actors/HitBox.HitBox_C" (`KismetMathLibrary.MakeTransform` (+ PositionOffset (.location (`Actor.GetTransform` (`self.GetOwner`)))) (.rotation (`Actor.GetTransform` (`self.GetOwner`))) (* (.scale (`Actor.GetTransform` (`self.GetOwner`))) (`local.Scalemultiply`))) "Undefined" "OverrideRootScale" null null))
  (bind _output_get (set `local.Created HB` _returnvalue_2))
  (set `/Game/Actors/HitBox.creator` _returnvalue _output_get)
  (set `/Game/Actors/HitBox.LaunchPow` LaunchPower _output_get)
  (set `/Game/Actors/HitBox.Damage` AttackPower _output_get)
  (`Actor.K2_AttachToActor` _output_get _returnvalue "None" "KeepWorld" "KeepRelative" "KeepRelative" true)
  (`KismetArrayLibrary.Array_Add` (`self.HitBoxes`) (`local.Created HB`)))