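; MechDoll is the modular mech displayed in the garage, rebuilt from the part choices stored in ProjectArmsInstance.
; BeginPlay builds the body, opens GarageCanvas, blends the player view and binds the canvas's attachment-change event to SetAttachment.
; SetAttachment looks up the slot's data table row by index, then applies its mesh and texture through a dynamic material, using MirroredMesh for the left arm.
; The initial build sets ArmR twice and never Legs.
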(event `self.ReceiveBeginPlay`
  (bind _returnvalue (`GameplayStatics.GetPlayerController` 0))
  (`self.Create Body`)
  (bind _returnvalue_2 (`|CreateWidget` "/Game/Widgets/GarageWidgets/GarageCanvas.GarageCanvas_C" _returnvalue))
  (`UserWidget.AddToViewport` _returnvalue_2 0)
  (add `/Game/Widgets/GarageWidgets/GarageCanvas.AttachmentChangeEvent` _returnvalue_2 (delegate `AttachmentChangeEvent_Event`))
  (`PlayerController.SetViewTargetWithBlend` _returnvalue null 0.1 "VTBlend_Linear" 0.0 false))

(event `AttachmentChangeEvent_Event`
  (params (SlotToChange :type "/Game/enums/AttachmentSlot Enum" :default "NewEnumerator0"))
  (`self.SetAttachment` SlotToChange))

(fn `Create Body`
  (locals (GI :type "Object Object Reference"))
  ;[1 1 1] add meshes
  (`self.SetAttachment` "NewEnumerator0")
  (`self.SetAttachment` "NewEnumerator1")
  (`self.SetAttachment` "NewEnumerator2")
  (`self.SetAttachment` "NewEnumerator2"))

(fn `Get DynamicMaterial`
  (params (Mesh :type "MeshComponent Object Reference"))
  (returns (DMI :type "MaterialInstanceDynamic Object Reference"))
  (bind _asmaterial_instance_dynamic (cast `MaterialInstanceDynamic` (`PrimitiveComponent.GetMaterial` Mesh 0)))
  (return _asmaterial_instance_dynamic))

(fn `SetAttachment`
  (params (AttachSlot :type "/Game/enums/AttachmentSlot Enum" :default "NewEnumerator0"))
  (locals (MeshtoChange :type "SkeletalMeshComponent Object Reference") (AttachType :type "/Game/enums/AttachmentType Enum") (FlipArm :type Boolean) (AttachIndex :type Integer) (TabletoRef :type "DataTable Object Reference") (NewMesh :type "SkeletalMesh Object Reference") (AttachTexture :type "Texture2D Object Reference") (Material :type "MaterialInstanceDynamic Object Reference"))
  (bind _tabletoref (`local.TabletoRef`))
  (bind _meshtochange (`local.MeshtoChange`))
  (bind _asproject_arms_instance (cast `ProjectArmsInstance` (`GameplayStatics.GetGameInstance`)))
  (switch `/Game/enums/AttachmentSlot` AttachSlot
    (:`NewEnumerator0`
      (set `local.AttachIndex` (`ProjectArmsInstance.CoreIndex` _asproject_arms_instance))
      (set `local.MeshtoChange` (`self.Core Mesh`))
      (set `local.TabletoRef` "/Game/Datatables/Cores.Cores")
      (set `local.AttachType` "NewEnumerator0"))
    (:`NewEnumerator1`
      (set `local.AttachIndex` (`ProjectArmsInstance.ArmLIndex` _asproject_arms_instance))
      (set `local.MeshtoChange` (`self.ArmLMesh`))
      (set `local.TabletoRef` "/Game/Datatables/Arms.Arms" :!label _label)
      (set `local.AttachType` "NewEnumerator1"))
    (:`NewEnumerator2`
      (set `local.AttachIndex` (`ProjectArmsInstance.ArmRIndex` _asproject_arms_instance))
      (set `local.MeshtoChange` (`self.ArmRMesh`))
      (set `local.FlipArm` true)
      (goto _label))
    (:`NewEnumerator3`
      (set `local.AttachIndex` (`ProjectArmsInstance.LegIndex` _asproject_arms_instance))
      (set `local.MeshtoChange` (`self.LegsMesh`))
      (set `local.TabletoRef` "/Game/Datatables/Legs.Legs")
      (set `local.AttachType` "NewEnumerator2")))
  (bind _outrownames (`DataTableFunctionLibrary.GetDataTableRowNames` _tabletoref))
  (switch `/Game/enums/AttachmentType` (`local.AttachType`)
    (:`NewEnumerator0`
      (bind _output (`|GetArrayItem` _outrownames (`local.AttachIndex`)))
      (bind _returnvalue (`|GetDataTableRow` _tabletoref _output)
        (:`then`
          (bind (_name _mesh _texture) (break `CoreAttachStruct` _returnvalue))
          (set `local.NewMesh` _mesh)
          (set `local.AttachTexture` _texture))))
    (:`NewEnumerator1`
      (bind _returnvalue_2 (`|GetDataTableRow` _tabletoref _output)
        (:`then`
          (if (`local.FlipArm`)
            (bind (_name_2 _mesh_2 _mirroredmesh _texture_2) (break `ArmAttachStruct` _returnvalue_2))
            (set `local.NewMesh` _mesh_2)
            (else
              (set `local.NewMesh` _mirroredmesh)))
          (set `local.AttachTexture` _texture_2))))
    (:`NewEnumerator2`
      (bind _returnvalue_3 (`|GetDataTableRow` _tabletoref _output)
        (:`then`
          (bind (_name_3 _mesh_3 _texture_3) (break `LegAttachStruct` _returnvalue_3))
          (set `local.NewMesh` _mesh_3)
          (set `local.AttachTexture` _texture_3)))))
  (`SkeletalMeshComponent.SetSkeletalMeshAsset` _meshtochange (`local.NewMesh`))
  (bind _returnvalue_4 (`PrimitiveComponent.CreateDynamicMaterialInstance` _meshtochange 0 "/Game/Materials/AttachmentMat.AttachmentMat" "None"))
  (bind _output_get (set `local.Material` _returnvalue_4))
  (`MaterialInstanceDynamic.SetTextureParameterValue` _output_get "BaseTex" (`local.AttachTexture`))
  (`PrimitiveComponent.SetMaterial` _meshtochange 0 (`local.Material`)))

(fn `UserConstructionScript`)