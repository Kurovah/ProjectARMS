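; Dummy is a hittable character that adds the damage it takes to the BattleManager's running total.
; On BeginPlay it caches the BattleManager and binds to the OnHit event of its HurtBox child actor, which forwards each hit context to GetHit.
; GetHit adds the damage, launches the character along Y away from the hit source, spawns a hit spark and prints the direction sign.
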(event `self.ReceiveBeginPlay`
  (bind _returnvalue (`GameplayStatics.GetActorOfClass` "/Game/Actors/BattleManager.BattleManager_C"))
  (set `self.Battle Manager` _returnvalue)
  (bind _ashurt_box (cast `/Game/Actors/HurtBox` (`ChildActorComponent.ChildActor` (`self.HurtBox`))))
  (add `/Game/Actors/HurtBox.OnHit` _ashurt_box (delegate `on Event`)))

(event `on Event`
  (params (HitContext :type "HitContext Structure"))
  (`self.GetHit` HitContext))

(fn `GetHit`
  (params (HitContext :type "HitContext Structure"))
  (bind (_sourceposition _damagevalue _launchvalue) (break `HitContext` HitContext))
  (bind _battle_manager (`self.Battle Manager`))
  (bind _returnvalue (`KismetMathLibrary.SignOfFloat` (- (`.Y` (`KismetMathLibrary.BreakVector3f` (`self.K2_GetActorLocation`))) (`.Y` (`KismetMathLibrary.BreakVector3f` _sourceposition)))))
  (set `/Game/Actors/BattleManager.Damage Applied` (+ _damagevalue (`/Game/Actors/BattleManager.Damage Applied` _battle_manager)) _battle_manager)
  (`KismetSystemLibrary.PrintString` (`KismetStringLibrary.Conv_DoubleToString` _returnvalue))
  (`self.LaunchCharacter` (`KismetMathLibrary.MakeVector` 0.0 (* _returnvalue _launchvalue)) true true)
  (`NiagaraFunctionLibrary.SpawnSystemAtLocation` "/Game/particle_systems/hitSpark.hitSpark" (`self.K2_GetActorLocation`)))

(fn `UserConstructionScript`)