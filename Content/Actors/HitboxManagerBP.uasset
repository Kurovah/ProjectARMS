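; Hitbox manager actor that creates and clears attack hitboxes on behalf of its parent actor.
; CreateHitBox spawns a HitBox, passes it the manager, creator, launch and attack power, then attaches it to the parent at a local offset.
; ClearHitboxes destroys tracked hitboxes and empties HitList, but removes array entries while iterating over them, which can skip some.
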(fn `ClearHitboxes`
  (locals (`actor to destroy` :type "/Game/Actors/HitBox Object Reference"))
  (bind _hitboxes (`self.HitBoxes`))
  (for _array_element _hitboxes
    (set `local.actor to destroy` _array_element)
    (`KismetArrayLibrary.Array_RemoveItem` _hitboxes _array_element)
    (`self.K2_DestroyActor` (`local.actor to destroy`))
    (`KismetArrayLibrary.Array_Clear` (`self.HitList`))))

(fn `CreateHitBox`
  (params (PositionOffset :type "Vector Structure") (LaunchPower :type "Float (double-precision)") (AttackPower :type "Float (double-precision)"))
  (bind _returnvalue (`self.GetParentActor`))
  (bind _returnvalue_2 (`|SpawnActorFromClass` "/Game/Actors/HitBox.HitBox_C" (`self.GetTransform` (`self.GetParentActor`)) "AlwaysSpawn" "OverrideRootScale" self null))
  (set `/Game/Actors/HitBox.Manager` self _returnvalue_2)
  (set `/Game/Actors/HitBox.creator` _returnvalue _returnvalue_2)
  (set `/Game/Actors/HitBox.launchStrength` LaunchPower _returnvalue_2)
  (set `/Game/Actors/HitBox.attackPower` AttackPower _returnvalue_2)
  (`self.K2_AttachToActor` _returnvalue_2 _returnvalue "None" "KeepWorld" "KeepRelative" "KeepRelative" true)
  (`self.K2_AddActorLocalOffset` _returnvalue_2 PositionOffset false false)
  (`KismetArrayLibrary.Array_Add` (`self.HitBoxes`) _returnvalue_2))

(fn `UserConstructionScript`)